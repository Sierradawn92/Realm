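; BP_LocationCard is an entrance trigger that shows a location-name card on the HUD when the player crosses it.
; Overlapping the collision copies LocationCardText to the ThirdPersonCharacter and toggles InZone, syncing it across OtherEntrances so an area's entrances share state.
; Only entering creates the LocationCard_HUD widget, plays its FadeIn and removes it after a delay.
; ResetCardEvent resets a DoOnce that the visible overlap flow does not use.
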(event `self.Collision.OnComponentBeginOverlap`
  (params (OverlappedComponent :type "PrimitiveComponent Object Reference") (OtherActor :type "Actor Object Reference") (OtherComp :type "PrimitiveComponent Object Reference") (OtherBodyIndex :type Integer) (bFromSweep :type Boolean) (SweepResult :type "HitResult Structure (by ref)"))
  (bind _otherentrances (`self.OtherEntrances`))
  (bind _asthird_person_character (cast `/Game/ThirdPersonBP/Blueprints/ThirdPersonCharacter` OtherActor))
  (set `/Game/ThirdPersonBP/Blueprints/ThirdPersonCharacter.LocationCardText` (`self.LocationCardText`) _asthird_person_character)
  (if (`self.InZone`)
    (for _array_element _otherentrances
      (set `/Game/HUD/BP_LocationCard.InZone` false _array_element))
    (set `self.InZone` false)
    (else
      (if (`KismetArrayLibrary.Array_IsValidIndex` _otherentrances)
        (for _array_element_2 _otherentrances
          (set `/Game/HUD/BP_LocationCard.InZone` true _array_element_2)))
      (set `self.InZone` true)
      (bind _returnvalue (`|CreateWidget` "/Game/HUD/Floor3_LocationCards/LocationCard_HUD.LocationCard_HUD_C"))
      (`UserWidget.AddToViewport` _returnvalue 0)
      (`UserWidget.PlayAnimation` _returnvalue (`/Game/HUD/Floor3_LocationCards/LocationCard_HUD.FadeIn` _returnvalue) 0.0 1 "Forward" 1.0)
      (`KismetSystemLibrary.Delay` 4.0)
      (`Widget.RemoveFromParent` _returnvalue))))

(event `ResetCardEvent`
  (`/Engine/EditorBlueprintResources/StandardMacros.DoOnce` false :!via `Reset`))

(fn `UserConstructionScript`)