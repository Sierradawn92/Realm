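; Elevator Blueprint whose sliding doors open for a third-person character carrying the required keycard.
; On trigger overlap it searches the character's owned keycards and, on a match, copies that list into the game instance.
; Two timelines then lerp the left and right doors' relative locations.
; Ending any overlap reverses both timelines, with no actor or keycard check; the Blueprint has no cabin movement logic.
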(event `self.Trigger.OnComponentBeginOverlap`
  (params (OverlappedComponent :type "PrimitiveComponent Object Reference") (OtherActor :type "Actor Object Reference") (OtherComp :type "PrimitiveComponent Object Reference") (OtherBodyIndex :type Integer) (bFromSweep :type Boolean) (SweepResult :type "HitResult Structure (by ref)"))
  (bind _asthird_person_character (cast `/Game/ThirdPersonBP/Blueprints/ThirdPersonCharacter` OtherActor))
  (bind _ownedkeycard (`/Game/ThirdPersonBP/Blueprints/ThirdPersonCharacter.OwnedKeycard` _asthird_person_character))
  ;[1 1 1] Required Keycard
  (for _array_element _ownedkeycard
    (if (`|EnumEquality` _array_element (`self.RequiedKeycard`))
      (bind _asrealm_instance_test (cast `/Game/Realm_Instance_Test` (`GameplayStatics.GetGameInstance`)))
      (set `/Game/Realm_Instance_Test.PlayerKeycard` _ownedkeycard _asrealm_instance_test)
      ;[1 1 1] Open
      (`|ExecutionSequence`
        (:`then_0`
          (bind (_direction _movement_left) (`Timeline|Movement_Left` :!label _label)
            (:`Update`
              (`SceneComponent.K2_SetRelativeLocation` (`self.SlideDoorLeft`) (`KismetMathLibrary.VLerp` (-70.0 -10.0 0.0) (40.0 -10.0 0.0) _movement_left) false false))))
        (:`then_1`
          (bind (_direction_2 _movement_left_2) (`Timeline|Movement_Right` :!label _label_2)
            (:`Update`
              (`SceneComponent.K2_SetRelativeLocation` (`self.SlideDoorRight`) (`KismetMathLibrary.VLerp` (470.0 -10.0 0.0) (360.0 -10.0 0.0) _movement_left_2) false false))))))))

(event `self.Trigger.OnComponentEndOverlap`
  (params (OverlappedComponent :type "PrimitiveComponent Object Reference") (OtherActor :type "Actor Object Reference") (OtherComp :type "PrimitiveComponent Object Reference") (OtherBodyIndex :type Integer))
  ;[1 1 1] Open
  (`|ExecutionSequence`
    (:`then_0`
      (goto _label :!via `Reverse`))
    (:`then_1`
      (goto _label_2 :!via `Reverse`))))

(fn `UserConstructionScript`)