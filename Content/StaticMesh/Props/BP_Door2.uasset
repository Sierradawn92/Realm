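; BP_Door2 is a double sliding door that moves when something overlaps its Collison component and moves back when the overlap ends.
; Begin overlap plays two timelines that lerp the relative locations of SMDoor and SMDoor2 along X in mirrored directions, and end overlap reverses both.
; The overlap events do not filter by actor or count occupants, so any end overlap reverses the doors.
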(event `self.Collison.OnComponentBeginOverlap`
  (params (OverlappedComponent :type "PrimitiveComponent Object Reference") (OtherActor :type "Actor Object Reference") (OtherComp :type "PrimitiveComponent Object Reference") (OtherBodyIndex :type Integer) (bFromSweep :type Boolean) (SweepResult :type "HitResult Structure (by ref)"))
  (`|ExecutionSequence`
    (:`then_0`
      (bind (_direction _newtrack_0) (`Timeline|Door1` :!label _label)
        (:`Update`
          (`SceneComponent.K2_SetRelativeLocation` (`self.SM_Door`) (`KismetMathLibrary.VLerp` (200.0 0.0 0.0) (101.0 0.0 0.0) _newtrack_0) false false))))
    (:`then_1`
      (bind (_direction_2 _newtrack_0_2) (`Timeline|Door2` :!label _label_2)
        (:`Update`
          (`SceneComponent.K2_SetRelativeLocation` (`self.SM_Door2`) (`KismetMathLibrary.VLerp` (-200.0 0.0 0.0) (-98.0 0.0 0.0) _newtrack_0_2) false false))))))

(event `self.Collison.OnComponentEndOverlap`
  (params (OverlappedComponent :type "PrimitiveComponent Object Reference") (OtherActor :type "Actor Object Reference") (OtherComp :type "PrimitiveComponent Object Reference") (OtherBodyIndex :type Integer))
  (`|ExecutionSequence`
    (:`then_0`
      (goto _label :!via `Reverse`))
    (:`then_1`
      (goto _label_2 :!via `Reverse`))))

(fn `UserConstructionScript`)