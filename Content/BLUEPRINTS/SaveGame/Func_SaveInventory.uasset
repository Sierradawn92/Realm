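; Blueprint functions that restore player progress from the "CurrentProgress" save slot; despite the asset's name, they only load.
; LoadLevelFunc teleports the character to the saved spawn transform and copies it to the game mode, using the character's current transform when no save or spawn is set.
; GetInventory restores keycard, ammo and health to the character, but casts the slot to BP_SaveGame, whereas LoadLevelFunc expects SG_SaveGame.
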(fn `GetInventory`
  (bind _returnvalue (`GameplayStatics.LoadGameFromSlot` "CurrentProgress"))
  (bind _asbp_save_game (cast `/Game/BLUEPRINTS/SaveGame/BP_SaveGame` _returnvalue))
  (bind _asthird_person_character (cast `/Game/ThirdPersonBP/Blueprints/ThirdPersonCharacter` (`GameplayStatics.GetPlayerCharacter` null)))
  (set `/Game/ThirdPersonBP/Blueprints/ThirdPersonCharacter.OwnedKeycard` (`/Game/BLUEPRINTS/SaveGame/BP_SaveGame.OwnedKeycard` _asbp_save_game) _asthird_person_character)
  (set `/Game/ThirdPersonBP/Blueprints/ThirdPersonCharacter.Ammo` (`/Game/BLUEPRINTS/SaveGame/BP_SaveGame.Ammo` _asbp_save_game) _asthird_person_character)
  (set `/Game/ThirdPersonBP/Blueprints/ThirdPersonCharacter.MaxAmmo` (`/Game/BLUEPRINTS/SaveGame/BP_SaveGame.MaxAmmo` _asbp_save_game) _asthird_person_character)
  (set `/Game/ThirdPersonBP/Blueprints/ThirdPersonCharacter.Health` (`/Game/BLUEPRINTS/SaveGame/BP_SaveGame.Health` _asbp_save_game) _asthird_person_character)
  (set `/Game/ThirdPersonBP/Blueprints/ThirdPersonCharacter.MaxHealth` (`/Game/BLUEPRINTS/SaveGame/BP_SaveGame.MaxHealth` _asbp_save_game) _asthird_person_character))

(fn `LoadLevelFunc`
  (locals (ThirdPersonCharacter :type "/Game/ThirdPersonBP/Blueprints/ThirdPersonCharacter Object Reference") (ThirdPersonGameMode :type "/Game/ThirdPersonBP/Blueprints/ThirdPersonGameMode Object Reference") (SaveGameRef :type "/Game/BLUEPRINTS/SaveGame/SG_SaveGame Object Reference"))
  (bind (_returnvalue_location _returnvalue_rotation) (`KismetMathLibrary.BreakTransform` (`Actor.GetTransform` (`local.ThirdPersonCharacter`))))
  (bind (_levelinfo_currentlevel _levelinfo_spawntransform) (break `/Game/BLUEPRINTS/SaveGame/ST_LevelInfo` (`/Game/BLUEPRINTS/SaveGame/SG_SaveGame.LevelInfo` (`local.SaveGameRef`))))
  (bind _asthird_person_character (cast `/Game/ThirdPersonBP/Blueprints/ThirdPersonCharacter` (`GameplayStatics.GetPlayerCharacter` null)))
  (set `local.ThirdPersonCharacter` _asthird_person_character)
  (bind _asthird_person_game_mode (cast `/Game/ThirdPersonBP/Blueprints/ThirdPersonGameMode` (`GameplayStatics.GetGameMode` null)))
  (set `local.ThirdPersonGameMode` _asthird_person_game_mode)
  (bind _returnvalue (`GameplayStatics.DoesSaveGameExist` "CurrentProgress"))
  (if _returnvalue
    (bind _returnvalue_2 (`GameplayStatics.LoadGameFromSlot` "CurrentProgress"))
    (bind _assg_save_game (cast `/Game/BLUEPRINTS/SaveGame/SG_SaveGame` _returnvalue_2))
    (bind _output_get (set `local.SaveGameRef` _assg_save_game))
    (bind (_levelinfo_currentlevel_2 _levelinfo_spawntransform_2) (break `/Game/BLUEPRINTS/SaveGame/ST_LevelInfo` (`/Game/BLUEPRINTS/SaveGame/SG_SaveGame.LevelInfo` _output_get)))
    (if (== _levelinfo_spawntransform_2 (`KismetMathLibrary.MakeTransform` (0.0 0.0 0.0)))
      (set `/Game/ThirdPersonBP/Blueprints/ThirdPersonGameMode.SpawnTransform` (`KismetMathLibrary.MakeTransform` _returnvalue_location _returnvalue_rotation) (`local.ThirdPersonGameMode`) :!label _label)
      (else
        (set `/Game/ThirdPersonBP/Blueprints/ThirdPersonGameMode.SpawnTransform` _levelinfo_spawntransform (`local.ThirdPersonGameMode`))
        (`Actor.K2_TeleportTo` (`local.ThirdPersonCharacter`) (.location _levelinfo_spawntransform) (.rotation _levelinfo_spawntransform))))
    (else
      (goto _label))))